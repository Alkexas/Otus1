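; Melee enemy bot that attacks player characters, takes damage and can drop a health pickup on death.
; BotAttack starts a looping timer that box-traces between the weapon's Tip and Base sockets, damaging Character-tagged actors with a DoOnce and Delay cooldown.
; AnyDamage updates the health component and widget, plays effects, then on zero health destroys the bot, rolls loot and calls MeleeDeath.
; An overlap volume shows the health widget while a character is nearby.
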(event OnComponentBeginOverlap(ShowHealth)
  (params (OverlappedComponent :type Primitive%20Component%20Object%20Reference) (OtherActor :type Actor%20Object%20Reference) (OtherComp :type Primitive%20Component%20Object%20Reference) (OtherBodyIndex :type Integer) (bFromSweep :type Boolean) (SweepResult :type Hit%20Result%20Structure%20%28by%20ref%29))
  ;[1 1 1] Health Sphere
  (if (Actor|ActorHasTag OtherActor "Character")
    (Development|SetHiddeninGame (Variables|Default|GetWidgetHealth) false false)))

(event OnComponentEndOverlap(ShowHealth)
  (params (OverlappedComponent :type Primitive%20Component%20Object%20Reference) (OtherActor :type Actor%20Object%20Reference) (OtherComp :type Primitive%20Component%20Object%20Reference) (OtherBodyIndex :type Integer))
  ;[1 1 1] Health Sphere
  (if (Actor|ActorHasTag OtherActor "Character")
    (Development|SetHiddeninGame (Variables|Default|GetWidgetHealth) true false)))

(event Custom|DropLoot
  (if (>= (Math|Random|RandomIntegerinRange 1 100) 50)
    (Game|SpawnActorfromClass "/Game/Assets/BP_Assets/BP_HealthPoint.BP_HealthPoint_C" (Math|Transform|MakeTransform (Transformation|GetActorLocation) "0, 0, 0" "1.000000,1.000000,1.000000") "Undefined" "MultiplyWithRoot" 0 0)))

(event Custom|BotAttack
  ;[1 0.476 0.476] Attack
  (Variables|Default|SetActive true)
  (Utilities|Time|SetTimerbyEvent (delegate Custom|AttackLineTrace) 0.1 true))

(event Custom|AttackLineTrace
  (bind _staticmesh (Variables|Default|GetStaticMesh))
  (bind _returnvalue (Transformation|GetSocketLocation _staticmesh "Base"))
  (bind _returnvalue_2 (Transformation|GetSocketLocation _staticmesh "Tip"))
  ;[1 0.476 0.476] Attack
  (if (Variables|Default|GetActive)
    (bind _outhit (Collision|BoxTraceByChannel _returnvalue_2 _returnvalue (Math|Vector|MakeVector (/ (Math|Vector|Distance(Vector) _returnvalue_2 _returnvalue) 2.0) 2e+01 5.0) (Math|Rotator|FindLookatRotation _returnvalue_2 _returnvalue) "TraceTypeQuery1" false 0 "None"))
    (if (.bBlockingHit (Collision|BreakHitResult _outhit))
      (if (Actor|ActorHasTag (.HitActor (Collision|BreakHitResult _outhit)) "Character")
        (Utilities|FlowControl|DoOnce false :!label _label
          (:Completed
            (Game|Damage|ApplyDamage (.HitActor (Collision|BreakHitResult _outhit)) 5.0 0 0)
            (Variables|Default|SetActive false)
            (Utilities|FlowControl|Delay 0.7)
            (goto _label Reset)))))))

(event Game|Damage|EventAnyDamage
  (params (Damage :type Float%20%28single-precision%29) (DamageType :type Damage%20Type%20Object%20Reference) (InstigatedBy :type Controller%20Object%20Reference) (DamageCauser :type Actor%20Object%20Reference))
  ;[0 1 0.02246] Damage
  (Default|GetDamage (Variables|Default|GetAC_Health) Damage)
  (Components|Activation|SetActive (Variables|Default|GetNiagara) true true)
  (Audio|PlaySound2D "/Game/Sound/Enemy/SC_EnemyDamage.SC_EnemyDamage" 1.0 1.0 0.0 0 0)
  (Audio|PlaySound2D "/Game/Sound/Weapon/SC_Rasrez.SC_Rasrez" 1.0 1.0 0.0 0 0)
  (CallFunction|DamageEnemy)
  (if (<= (Variables|/Game/Components/AC_Health.AC_Health_C|GetHealth (Variables|Default|GetAC_Health)) 0.0)
    (Actor|DestroyActor)
    (CallFunction|DropLoot)
    (Default|CallMeleeDeath)))

(event EventBeginPlay)

(event EventDamageEnemy
  ;[0 1 0.02246] Damage
  (Class|BPEnemyInterface|SetHealth(Message) (UserInterface|GetUserWidgetObject (Variables|Default|GetWidgetHealth)) (stale Game|Damage|EventAnyDamage Damage)))

(fn ConstructionScript)

(fn GetMesh
  (return 0))

(fn GetHealth
  (return 0.0))