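; BP_BotRange is a ranged enemy bot that fires arrows from a mesh socket after a short delay.
; Damage feeds a health component, triggers Niagara and sound effects, and updates a health widget that shows only while a Character-tagged actor overlaps its sphere.
; At zero health it destroys itself, has a roughly even chance to drop health and arrow pickups together, and calls RangeDeath.
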(event OnComponentBeginOverlap(ShowHealth)
  (params (OverlappedComponent :type Primitive%20Component%20Object%20Reference) (OtherActor :type Actor%20Object%20Reference) (OtherComp :type Primitive%20Component%20Object%20Reference) (OtherBodyIndex :type Integer) (bFromSweep :type Boolean) (SweepResult :type Hit%20Result%20Structure%20%28by%20ref%29))
  ;[1 1 1] Health Sphere
  (if (Actor|ActorHasTag OtherActor "Character")
    (Development|SetHiddeninGame (Variables|Default|GetWidget%20Health) false false)))

(event OnComponentEndOverlap(ShowHealth)
  (params (OverlappedComponent :type Primitive%20Component%20Object%20Reference) (OtherActor :type Actor%20Object%20Reference) (OtherComp :type Primitive%20Component%20Object%20Reference) (OtherBodyIndex :type Integer))
  ;[1 1 1] Health Sphere
  (if (Actor|ActorHasTag OtherActor "Character")
    (Development|SetHiddeninGame (Variables|Default|GetWidget%20Health) true false)))

(event Custom|DropLoot
  (bind _returnvalue (Transformation|GetActorLocation))
  (if (>= (Math|Random|RandomIntegerinRange 1 100) 50)
    (Game|SpawnActorfromClass "/Game/Assets/BP_Assets/BP_HealthPoint.BP_HealthPoint_C" (Math|Transform|MakeTransform _returnvalue "0, 0, 0" "1.000000,1.000000,1.000000") "AlwaysSpawn" "MultiplyWithRoot" 0 0)
    (Game|SpawnActorfromClass "/Game/Assets/BP_Assets/BP_ArrowCounter.BP_ArrowCounter_C" (Math|Transform|MakeTransform (+ _returnvalue "10.000000,5.000000,0.000000") "0, 0, 0" "1.000000,1.000000,1.000000") "AlwaysSpawn" "MultiplyWithRoot" 0 0)))

(event Custom|ShootArrow
  (Utilities|FlowControl|Delay 0.5)
  (Game|SpawnActorfromClass "/Game/AI/BP_ArrowBot.BP_ArrowBot_C" (Transformation|GetSocketTransform (Variables|Character|GetMesh) "ArrowSlot" "RTS_World") "AdjustIfPossibleButAlwaysSpawn" "MultiplyWithRoot" 0 0))

(event Game|Damage|EventAnyDamage
  (params (Damage :type Float%20%28single-precision%29) (DamageType :type Damage%20Type%20Object%20Reference) (InstigatedBy :type Controller%20Object%20Reference) (DamageCauser :type Actor%20Object%20Reference))
  ;[1 0 0] Damage
  (Default|GetDamage (Variables|Default|GetAC_Health) Damage)
  (Components|Activation|SetActive (Variables|Default|GetNiagara) true true)
  (Audio|PlaySound2D "/Game/Sound/Enemy/SC_EnemyDamage.SC_EnemyDamage" 1.0 1.0 0.0 0 0)
  (Audio|PlaySound2D "/Game/Sound/Weapon/SC_Rasrez.SC_Rasrez" 1.0 1.0 0.0 0 0)
  (CallFunction|DamageEnemy)
  (if (<= (Variables|/Game/Components/AC_Health.AC_Health_C|GetHealth (Variables|Default|GetAC_Health)) 0.0)
    (Actor|DestroyActor)
    (CallFunction|DropLoot)
    (Default|CallRangeDeath)))

(event EventDamageEnemy
  ;[1 0 0] Damage
  (Class|BPEnemyInterface|SetHealth(Message) (UserInterface|GetUserWidgetObject (Variables|Default|GetWidget%20Health)) (stale Game|Damage|EventAnyDamage Damage)))

(fn ConstructionScript)

(fn GetHealth
  (return 0.0))