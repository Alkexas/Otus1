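; BP_ArrowBot is an arrow projectile, filed under AI, that damages and sticks into what it hits.
; When SticToActor first overlaps another actor, it destroys the projectile movement, enables collision and attaches to the swept hit component, keeping world transform.
; It then sets a short lifespan and applies flat damage to the sweep's hit actor.
; An FS_Damage spawn and trigger is left unconnected and never runs.
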(event OnComponentBeginOverlap(Stictoactor)
  (params (OverlappedComponent :type Primitive%20Component%20Object%20Reference) (OtherActor :type Actor%20Object%20Reference) (OtherComp :type Primitive%20Component%20Object%20Reference) (OtherBodyIndex :type Integer) (bFromSweep :type Boolean) (SweepResult :type Hit%20Result%20Structure%20%28by%20ref%29))
  (bind (_bblockinghit _binitialoverlap _time _distance _location _impactpoint _normal _impactnormal _physmat _hitactor _hitcomponent) (Collision|BreakHitResult SweepResult))
  (if (!= OtherActor self)
    (bind _projectilemovement (Variables|Default|GetProjectileMovement)
      (:then
        (Components|DestroyComponent _projectilemovement)
        (Collision|SetCollisionEnabled (Variables|Default|GetStic%20to%20actor) "QueryAndPhysics")
        (Transformation|AttachComponentToComponent _hitcomponent "None" "KeepWorld" "KeepWorld" "KeepWorld" true)
        (Actor|SetLifeSpan 3.0)
        (Game|Damage|ApplyDamage _hitactor 25.0 0 0))
      (:else))))

(fn ConstructionScript)