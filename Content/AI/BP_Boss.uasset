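; Dragon boss character with flame and slash attacks, plus a health bar shown while the player is inside its proximity sphere.
; Each attack plays a montage and starts looping timers that box-trace from head or hand to apply damage.
; Slash also activates Niagara effects and launches the player through a forward sphere trace.
; Incoming damage feeds ACBossHealth and the widget; at zero health the boss is destroyed and drops an item near the player.
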(event OnComponentBeginOverlap(Sphere)
  (params (OverlappedComponent :type Primitive%20Component%20Object%20Reference) (OtherActor :type Actor%20Object%20Reference) (OtherComp :type Primitive%20Component%20Object%20Reference) (OtherBodyIndex :type Integer) (bFromSweep :type Boolean) (SweepResult :type Hit%20Result%20Structure%20%28by%20ref%29))
  ;[0 0.06178 1] Widget
  (if (Actor|ActorHasTag OtherActor "Character")
    (Widget|SetVisibility (Variables|Default|GetWidgetHealth) "Visible")))

(event OnComponentEndOverlap(Sphere)
  (params (OverlappedComponent :type Primitive%20Component%20Object%20Reference) (OtherActor :type Actor%20Object%20Reference) (OtherComp :type Primitive%20Component%20Object%20Reference) (OtherBodyIndex :type Integer))
  ;[0 0.06178 1] Widget
  (if (Actor|ActorHasTag OtherActor "Character")
    (Widget|SetVisibility (Variables|Default|GetWidgetHealth) "Hidden")))

(event Custom|Flame
  (bind _headsphere (Variables|Default|GetHeadSphere))
  (bind _returnvalue (Transformation|GetWorldLocation _headsphere))
  ;[1 0 0] AttackFlame
  (if (Variables|Default|GetActiveFlame)
    (bind _outhit (Collision|BoxTraceByChannel _returnvalue (+ _returnvalue (* (Variables|Default|GetLength) (Math|Vector|GetForwardVector _headsphere))) "100.000000,0.000000,70.000000" "0, 0, 0" "TraceTypeQuery1" false 0 "None"))
    (if (.bBlockingHit (Collision|BreakHitResult _outhit))
      (Game|Damage|ApplyDamage (.HitActor (Collision|BreakHitResult _outhit)) 1.0 0 self)
      (Variables|Default|SetActiveFlame false))))

(event Custom|Montage
  ;[1 0 0] AttackFlame
  (Variables|Default|SetActiveFlame true)
  (Utilities|Time|SetTimerbyEvent (delegate Custom|Flame) 0.1 true true))

(event Custom|DragonFlame
  ;[1 0 0] AttackFlame
  (Animation|PlayAnimMontage "/Game/AI/Boss/Animation/AS_DragonFlame_Montage.AS_DragonFlame_Montage" 1.0 "None")
  (Utilities|FlowControl|Delay 3.0)
  (Audio|PlaySound2D "/Game/Sound/Enemy/SC_DragonFlame.SC_DragonFlame" 1.0 1.0 0.0 0 0)
  (CallFunction|Montage)
  (Utilities|FlowControl|Delay 5.0)
  (Animation|StopAnimMontage "/Game/AI/Boss/Animation/AS_DragonFlame_Montage.AS_DragonFlame_Montage")
  (Utilities|FlowControl|DoOnce false :!label _label
    (:Completed
      (Utilities|Time|PauseTimerbyHandle)
      (goto _label Reset))))

(event Custom|DragonSlash
  ;[0.6781 0 0] DragonSlash
  (Audio|PlaySound2D "/Game/Sound/Enemy/SC_DragonRoar.SC_DragonRoar" 1.0 1.0 0.0 0 0)
  (Animation|PlayAnimMontage "/Game/AI/Boss/Animation/AS_DragonSlash_Montage.AS_DragonSlash_Montage" 1.0 "None")
  (Utilities|FlowControl|Delay 0.7)
  (CallFunction|PushChar)
  (Utilities|FlowControl|Delay 0.7)
  (Components|Activation|SetActive (Variables|Default|GetNiagara) true true)
  (Variables|Default|SetActiveSlash true)
  (Utilities|Time|SetTimerbyEvent (delegate Custom|Slash) 0.1 true))

(event Custom|Widget
  ;[0 0.06178 1] Widget
  (bind _returnvalue (UserInterface|CreateWidget "/Game/UI/WB_BossHealth.WB_BossHealth_C"))
  (bind _output_get (Variables|Default|SetWidgetHealth _returnvalue))
  (UserInterface|Viewport|AddtoViewport _output_get 0)
  (Widget|SetVisibility _output_get "Hidden"))

(event Custom|Slash
  (bind _handcube (Variables|Default|GetHandCube))
  (bind _returnvalue (Transformation|GetWorldLocation _handcube))
  ;[0.6781 0 0] DragonSlash
  (if (Variables|Default|GetActiveSlash)
    (bind _outhit (Collision|BoxTraceByChannel _returnvalue (+ _returnvalue (* (Variables|Default|GetLengthHand) (Math|Vector|GetForwardVector _handcube))) "50.000000,10.000000,50.000000" "0, 0, 0" "TraceTypeQuery1" false 0 "None"))
    (if (.bBlockingHit (Collision|BreakHitResult _outhit))
      (Utilities|FlowControl|DoOnce false :!label _label
        (:Completed
          (Game|Damage|ApplyDamage (.HitActor (Collision|BreakHitResult _outhit)) (Math|Random|RandomFloatinRange 5.0 15.0) 0 self)
          (Variables|Default|SetActiveSlash false)
          (Utilities|FlowControl|Delay 0.5)
          (goto _label Reset))))))

(event Custom|PushChar
  (bind _capsulecomponent (Variables|Collision|GetCapsuleComponent))
  (bind _capsulecomponent_2 (Variables|Collision|GetCapsuleComponent))
  (bind _returnvalue (Transformation|GetWorldLocation _capsulecomponent_2))
  (bind _returnvalue_2 (Transformation|GetWorldRotation _capsulecomponent))
  (bind _returnvalue_3 (Math|Vector|GetForwardVector _returnvalue_2))
  (bind _returnvalue_4 (* _returnvalue_3 1e+03))
  ;[0 1 0.9354] Push
  (Utilities|FlowControl|Delay 0.7)
  (bind (_outhit _returnvalue_5) (Collision|SphereTraceByChannel _returnvalue (+ _returnvalue (* (Math|Vector|GetForwardVector (Transformation|GetWorldRotation _capsulecomponent_2)) 1e+03)) 1e+02 "TraceTypeQuery1" false 0 "None"))
  (if _returnvalue_5
    (bind _asbp_kunaiji (Utilities|Casting|CastToBP_Kunaiji (.HitActor (Collision|BreakHitResult _outhit))))
    (Character|LaunchCharacter _asbp_kunaiji (Math|Vector|MakeVector (.x _returnvalue_4) (.y _returnvalue_4) (+ (.z _returnvalue_4) 5e+02)) false false)))

(event Custom|CharRef
  ;[1 1 1] BeginPlay
  (bind _asbp_kunaiji (Utilities|Casting|CastToBP_Kunaiji (Game|GetPlayerCharacter 0)))
  (Variables|Default|SetKunajiRef _asbp_kunaiji))

(event Game|Damage|EventAnyDamage
  (params (Damage :type Float%20%28single-precision%29) (DamageType :type Damage%20Type%20Object%20Reference) (InstigatedBy :type Controller%20Object%20Reference) (DamageCauser :type Actor%20Object%20Reference))
  (bind _kunajiref (Variables|Default|GetKunajiRef))
  (bind _rootcomponent (Variables|/Script/Engine.Actor|GetRootComponent _kunajiref))
  (bind _returnvalue (Transformation|GetWorldLocation _rootcomponent))
  (bind _returnvalue_2 (Transformation|GetWorldRotation _rootcomponent))
  (bind _returnvalue_3 (* _returnvalue_2 1e+02))
  (bind _returnvalue_4 (+ _returnvalue _returnvalue_3))
  ;[1 0.2421 0] TakeDamage
  (Default|GetDamage (Variables|Default|GetAC_BossHealth) Damage)
  (CallFunction|DamageEnemy)
  (Audio|PlaySound2D "/Game/Sound/Weapon/SC_Rasrez.SC_Rasrez" 1.0 1.0 0.0 0 0)
  (if (<= (Variables|/Game/Components/AC_BossHealth.AC_BossHealth_C|GetHealth (Variables|Default|GetAC_BossHealth)) 0.0)
    (Actor|DestroyActor)
    ;[1 0.6304 0] Drop Item
    (Game|SpawnActorfromClass "/Game/Inventory/BP/BP_Item.BP_Item_C" (Math|Transform|MakeTransform _returnvalue_4 "0, 0, 0" "1.000000,1.000000,1.000000") "Undefined" "MultiplyWithRoot" 0 (Variables|Default|GetItem) 0)
    (Audio|PlaySoundatLocation "/Engine/VREditor/Sounds/UI/Camera_Shutter.Camera_Shutter" _returnvalue_4 "0, 0, 0" 1.0 1.0 0.0 0 0 0 0)))

(event EventDamageEnemy
  ;[1 0.2421 0] TakeDamage
  (Class|BPEnemyInterface|SetHealth(Message) (Variables|Default|GetWidgetHealth) (stale Game|Damage|EventAnyDamage Damage)))

(event EventBeginPlay
  ;[1 1 1] BeginPlay
  (CallFunction|Widget)
  (CallFunction|CharRef))

(fn ConstructionScript)

(fn GetMesh
  (return 0))

(fn GetHealth
  (return 0.0))