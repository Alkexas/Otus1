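; AI controller for the boss that runs the BT_Boss behavior tree on BeginPlay and feeds it perception data through the Blackboard.
; Sight stimuli from the player set Enemy while seen, then clear it and store LastLocation when sight is lost.
; Hearing stimuli from any actor write their location to TargetPoint.
; Perception updates also print the names of updated actors, and GetMesh is an empty stub.
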(event OnTargetPerceptionUpdated(AIPerception)
  (params (Actor :type Actor%20Object%20Reference) (Stimulus :type AI%20Stimulus%20Structure))
  (CallFunction|HandleSightSense Actor Stimulus)
  (CallFunction|HandleSoundSense Stimulus))

(event OnPerceptionUpdated(AIPerception)
  (params (UpdatedActors :type Array%20of%20Actor%20Object%20References))
  (for _array_element UpdatedActors
    (Development|PrintString (Utilities|GetDisplayName _array_element))))

(event EventBeginPlay
  (AI|RunBehaviorTree "/Game/AI/BT_Boss.BT_Boss"))

(fn ConstructionScript)

(fn HandleSoundSense
  (params (Stimulus :type AI%20Stimulus%20Structure%20%28by%20ref%29))
  (bind _returnvalue (Class|AIPerceptionSystem|GetSenseClassforStimulus Stimulus))
  (if (== _returnvalue "/Script/AIModule.AISense_Hearing")
    (AI|Components|Blackboard|SetValueasVector (Variables|Default|GetBlackboard) (Utilities|Name|MakeLiteralName "TargetPoint") (.StimulusLocation (Utilities|Struct|BreakAIStimulus Stimulus)))))

(fn HandleSightSense
  (params (Actor :type Actor%20Object%20Reference) (Stimulus :type AI%20Stimulus%20Structure))
  (bind _returnvalue (Class|AIPerceptionSystem|GetSenseClassforStimulus Stimulus))
  (if (== _returnvalue "/Script/AIModule.AISense_Sight")
    (if (== Actor (Game|GetPlayerCharacter 0))
      (AI|Components|Blackboard|SetValueasObject (Variables|Default|GetBlackboard) (Utilities|Name|MakeLiteralName "Enemy") (Utilities|SelectObject (Game|GetPlayerCharacter 0) 0 (.bsuccessfullysensed (Variables|Default|GetStimulus))))
      (if (not (.bsuccessfullysensed (Variables|Default|GetStimulus)))
        (AI|Components|Blackboard|SetValueasVector (Variables|Default|GetBlackboard) (Utilities|Name|MakeLiteralName "LastLocation") (.stimuluslocation (Variables|Default|GetStimulus))))
      (else
        (return)))
    (else
      (return))))

(fn GetMesh
  (return 0))