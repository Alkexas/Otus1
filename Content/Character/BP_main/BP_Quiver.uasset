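; BP_Quiver is a quiver pickup that the player wears and that shows whether arrows remain.
; Interact attaches it to the player mesh's QuiverPlace socket and sets HasQuiver on BP_Kunaiji.
; Actor overlap destroys its capsule, adds the WB_WeaponHUD widget and sets its own HasQuiver.
; A looping timer polls BP_Kunaiji's ArrowCounter, hiding or showing all arrow components together.
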(event Custom|ArrowInQuiver
  (bind _arrow1 (Variables|Default|GetArrow1))
  (bind _returnvalue (Actor|GetActorOfClass "/Game/Character/BP_main/BP_Kunaiji.BP_Kunaiji_C"))
  (if (< (Variables|/Game/Character/BP_main/BP_Kunaiji.BP_Kunaiji_C|GetArrowCounter _returnvalue) 1)
    (Rendering|SetVisibility _arrow1 false false)
    (else
      (Rendering|SetVisibility _arrow1 true false))))

(event EventBeginPlay
  (Utilities|Time|SetTimerbyEvent (delegate Custom|ArrowInQuiver) 0.1 true true))

(event Collision|EventActorBeginOverlap
  (params (OtherActor :type Actor%20Object%20Reference))
  (Components|DestroyComponent (Variables|Default|GetCapsule))
  (bind _returnvalue (UserInterface|CreateWidget "/Game/UI/WB_WeaponHUD.WB_WeaponHUD_C"))
  (bind _output_get (Variables|Default|SetWeapon%20Widget _returnvalue))
  (UserInterface|Viewport|AddtoViewport _output_get 0)
  (Variables|Default|SetHasQuiver true))

(fn ConstructionScript)

(fn Interact
  (params (IsPickUp? :type Boolean))
  (Transformation|AttachComponentToComponent (Variables|/Script/Engine.Character|GetMesh (Game|GetPlayerCharacter 0)) "QuiverPlace" "SnapToTarget" "SnapToTarget" "KeepRelative" true)
  (bind _outactors (Actor|GetAllActorsOfClass "/Game/Character/BP_main/BP_Kunaiji.BP_Kunaiji_C"))
  (Variables|/Game/Character/BP_main/BP_Kunaiji.BP_Kunaiji_C|SetHas%20Quiver? (Utilities|Array|Get(acopy) _outactors) true)
  (return false))