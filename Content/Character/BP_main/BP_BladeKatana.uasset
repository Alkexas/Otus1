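; BP_BladeKatana is a katana weapon actor whose blade applies damage effects on contact.
; On BeginPlay it finds the BP_Kunaiji actor in the level and sets its HasBlock flag to true.
; Each blade overlap, with no filtering, spawns an FS_Damage actor at the blade's transform, sets its activation type and fires its CETrigger event.
; GetMesh exposes the blade component to other Blueprints.
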(event OnComponentBeginOverlap(blade_katana_0)
  (params (OverlappedComponent :type Primitive%20Component%20Object%20Reference) (OtherActor :type Actor%20Object%20Reference) (OtherComp :type Primitive%20Component%20Object%20Reference) (OtherBodyIndex :type Integer) (bFromSweep :type Boolean) (SweepResult :type Hit%20Result%20Structure%20%28by%20ref%29))
  (bind _blade_katana_0 (Variables|Default|Getblade_katana_0))
  (Utilities|FlowControl|Sequence
    (:then_0
      (bind _returnvalue (Game|SpawnActorfromClass "/Game/Character/Mesh_bow/FS_Damage.FS_Damage_C" (Math|Transform|MakeTransform (Transformation|GetWorldLocation _blade_katana_0) (Transformation|GetWorldRotation _blade_katana_0) "1.000000,1.000000,1.000000") "Undefined" "MultiplyWithRoot" 0 0))
      (Variables|/Game/Character/Mesh_bow/FS_Damage.FS_Damage_C|SetActivationType _returnvalue "NewEnumerator4")
      (Default|CETrigger _returnvalue))))

(event EventBeginPlay
  (bind _returnvalue (Actor|GetActorOfClass "/Game/Character/BP_main/BP_Kunaiji.BP_Kunaiji_C"))
  (Variables|/Game/Character/BP_main/BP_Kunaiji.BP_Kunaiji_C|SetHas%20Block _returnvalue true))

(fn ConstructionScript)

(fn GetMesh
  (return (Variables|Default|Getblade_katana_0)))