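; BP_Arrow is a fired arrow that damages and sticks to what it hits, caching its BP_Kunaiji owner on spawn.
; Fire adds a projectile movement component at runtime, sets its velocity along the given direction and offsets the arrow locally.
; The first valid overlap destroys that movement, attaches to the hit component, triggers a spawned FS_Damage actor, applies damage and starts a short lifespan.
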(event OnComponentBeginOverlap(Stictoactor)
  (params (OverlappedComponent :type Primitive%20Component%20Object%20Reference) (OtherActor :type Actor%20Object%20Reference) (OtherComp :type Primitive%20Component%20Object%20Reference) (OtherBodyIndex :type Integer) (bFromSweep :type Boolean) (SweepResult :type Hit%20Result%20Structure%20%28by%20ref%29))
  (bind (_bblockinghit _binitialoverlap _time _distance _location _impactpoint _normal _impactnormal _physmat _hitactor _hitcomponent) (Collision|BreakHitResult SweepResult))
  (bind _arrow (Variables|Default|GetArrow))
  (if (!= OtherActor self)
    (bind _projectilemovement (Variables|Default|GetProjectileMovement)
      (:then
        (Components|DestroyComponent _projectilemovement)
        (Collision|SetCollisionEnabled (Variables|Default|GetStic%20to%20actor) "QueryAndPhysics")
        (Transformation|AttachComponentToComponent _hitcomponent "None" "KeepWorld" "KeepWorld" "KeepWorld" true)
        (bind _returnvalue (Game|SpawnActorfromClass "/Game/Character/Mesh_bow/FS_Damage.FS_Damage_C" (Math|Transform|MakeTransform (Transformation|GetWorldLocation _arrow) (Transformation|GetWorldRotation _arrow) "0.500000,0.500000,0.500000") "Undefined" "MultiplyWithRoot" 0 0))
        (Variables|/Game/Character/Mesh_bow/FS_Damage.FS_Damage_C|SetActivationType _returnvalue "NewEnumerator4")
        (Default|CETrigger _returnvalue)
        (Actor|SetLifeSpan 3.0)
        (Game|Damage|ApplyDamage _hitactor 25.0 0 0))
      (:else))))

(event Custom|Fire
  (params (Direction :type Vector))
  (bind _returnvalue (AddComponent|AddProjectileMovementComponent))
  (bind _output_get (Variables|Default|SetProjectileMovement _returnvalue))
  (Variables|/Script/Engine.MovementComponent|SetVelocity _output_get (* Direction 5e+03))
  (Transformation|AddActorLocalOffset "0.000000,65.000000,25.000000" false false))

(event EventBeginPlay
  (bind _asbp_kunaiji (Utilities|Casting|CastToBP_Kunaiji (Components|GetOwner)))
  (Variables|Default|SetAs%20BP%20Kunaiji _asbp_kunaiji))

(fn ConstructionScript)