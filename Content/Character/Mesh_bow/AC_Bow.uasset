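; AC_Bow is a component on the BP_Kunaiji character that handles bow aiming state and equipping.
; It caches the owner at BeginPlay, and its AimBegin and AimEnd events toggle IsAiming and the EBow enum.
; EquipBow and UnEquipBow find a BP_Bow in the world via GetActorOfClass and snap it to the BowHand or BowPlace mesh socket.
; A spring-arm length setter is present but unconnected.
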(event Custom|AimBegin
  (Variables|Default|SetIsAiming true)
  (Variables|Default|SetE_Bow "NewEnumerator1"))

(event Custom|AimEnd
  (Variables|Default|SetIsAiming false)
  (Variables|Default|SetE_Bow "NewEnumerator0"))

(event EventBeginPlay
  (bind _asbp_kunaiji (Utilities|Casting|CastToBP_Kunaiji (Components|GetOwner)))
  (Variables|Default|SetAs%20BP%20Kunaiji _asbp_kunaiji))

(fn EquipBow
  (bind _returnvalue (Actor|GetActorOfClass "/Game/Character/Mesh_bow/BP_Bow.BP_Bow_C"))
  (bind _output_get (Variables|Default|SetBow _returnvalue))
  (Transformation|AttachComponentToComponent _output_get (Variables|/Script/Engine.Character|GetMesh (Variables|Default|GetAs%20BP%20Kunaiji)) "BowHand" "SnapToTarget" "SnapToTarget" "KeepRelative" true))

(fn UnEquipBow
  (bind _returnvalue (Actor|GetActorOfClass "/Game/Character/Mesh_bow/BP_Bow.BP_Bow_C"))
  (bind _output_get (Variables|Default|SetBow _returnvalue))
  (Transformation|AttachComponentToComponent _output_get (Variables|/Script/Engine.Character|GetMesh (Variables|Default|GetAs%20BP%20Kunaiji)) "BowPlace" "SnapToTarget" "SnapToTarget" "KeepRelative" true))