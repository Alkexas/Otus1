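; Player controller for an inventory system that creates the main HUD widget on BeginPlay and bridges item slot changes to the UI.
; InventoryShow toggles inventory visibility, mouse cursor and input mode, though its only call here is in unreachable logic.
; UpdateItemSlot and ResetItemSlot forward to the indexed slot in one hardcoded container grid, ignoring their Container argument.
; PlayerControllerRef returns the controller itself.
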(event Custom|UpdateItemSlot
  (params (Index :type Integer) (ItemInfo :type S%20Item%20Info%20Structure) (Container :type E_Container%20Enum :default "NewEnumerator0"))
  (bind _mainref (Variables|Default|GetMainRef))
  (bind _wb_newinventory (Variables|/Game/X_NewInventory/Widgets/WB_Main.WB_Main_C|GetWB_NewInventory _mainref))
  (bind _wb_containergrid_259 (Variables|/Game/X_NewInventory/Widgets/WB_NewInventory.WB_NewInventory_C|GetWB_ContainerGrid_259 _wb_newinventory))
  (bind _slots (Variables|/Game/X_NewInventory/Widgets/WB_ContainerGrid.WB_ContainerGrid_C|GetSlots _wb_containergrid_259))
  (bind _output (Utilities|Array|Get(acopy) _slots Index))
  (Utilities|IsValid _output
    (:Is%20Valid
      (Default|UpdateSlotEvent _output ItemInfo))))

(event Custom|InventoryShow
  (bind _returnvalue (Game|GetPlayerController 0))
  (bind _mainref (Variables|Default|GetMainRef))
  (if (Variables|Default|GetInventoryShow?)
    (Default|IntentoryVisible _mainref false)
    (Variables|Default|SetInventoryShow? false)
    (Variables|/Script/Engine.PlayerController|SetbShowMouseCursor _returnvalue false)
    (Input|SetInputModeGameOnly _returnvalue false)
    (else
      (Default|IntentoryVisible _mainref true)
      (Variables|Default|SetInventoryShow? true)
      (Variables|/Script/Engine.PlayerController|SetbShowMouseCursor _returnvalue true)
      (Input|SetInputModeGameandUI _returnvalue 0 "DoNotLock" true false))))

(event Custom|ResetItemSlot
  (params (Container :type E_Container%20Enum :default "NewEnumerator0") (Index :type Integer))
  (bind _mainref (Variables|Default|GetMainRef))
  (bind _wb_newinventory (Variables|/Game/X_NewInventory/Widgets/WB_Main.WB_Main_C|GetWB_NewInventory _mainref))
  (bind _wb_containergrid_259 (Variables|/Game/X_NewInventory/Widgets/WB_NewInventory.WB_NewInventory_C|GetWB_ContainerGrid_259 _wb_newinventory))
  (bind _slots (Variables|/Game/X_NewInventory/Widgets/WB_ContainerGrid.WB_ContainerGrid_C|GetSlots _wb_containergrid_259))
  (bind _output (Utilities|Array|Get(acopy) _slots Index))
  (Utilities|IsValid _output
    (:Is%20Valid
      (Default|ResetSlot _output))))

(event EventBeginPlay
  (bind _returnvalue (UserInterface|CreateWidget "/Game/X_NewInventory/Widgets/WB_Main.WB_Main_C" self))
  (bind _output_get (Variables|Default|SetMainRef _returnvalue))
  (UserInterface|Viewport|AddtoViewport _output_get 0))

(event Input|KeyboardEvents|Tab
  (params (Key :type Key%20Structure :default "None")))

(fn ConstructionScript)

(fn PlayerControllerRef
  (return self))