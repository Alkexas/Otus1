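; Player inventory component that extends a parent container class with drag-and-drop handling and slot UI notifications.
; HandleSlotDrop has the source container transfer the dragged item into this inventory at the dropped index.
; Add and remove overrides run the parent logic, then message the owner's controller/character interface to update or reset the matching slot, identified by container type and index.
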(fn HandleSlotDrop
  (params (FromContainer :type BPC%20Item%20Container%20Object%20Reference) (FromIndex :type Integer) (DroppedIndex :type Integer))
  (LocalVariables|SetLocalFromContainer FromContainer)
  (LocalVariables|SetLocalFromIndex FromIndex)
  (LocalVariables|SetLocalDroppedIndex DroppedIndex)
  (switch Utilities|FlowControl|Switch|SwitchonE_Container (Variables|/Game/X_NewInventory/Classes/BPC_Item_Container.BPC_Item_Container_C|GetContainerType (LocalVariables|GetLocalFromContainer))
    (:NewEnumerator0
      (Default|TransferItem (LocalVariables|GetLocalFromContainer) self (LocalVariables|GetLocalDroppedIndex) (LocalVariables|GetLocalFromIndex)))))

(fn AddItemtoIndex
  (params (Item :type S%20Item%20Info%20Structure) (LocalSpecificalIndex :type Integer) (FromIndex :type Integer))
  (bind _success_ (|CallParentFunction Item LocalSpecificalIndex FromIndex))
  (bind _controllerref (Class|BPICharacter|GetControllerCharacter(Message) (Components|GetOwner)))
  (Default|UpdateItemSlot _controllerref LocalSpecificalIndex (CallFunction|GetItematIndex LocalSpecificalIndex) (Variables|Default|GetContainerType))
  (return _success_))

(fn RemoveItematIndex
  (params (Index :type Integer))
  (bind _success_ (|CallParentFunction Index))
  (bind _controllerref (Class|BPICharacter|GetControllerCharacter(Message) (Components|GetOwner)))
  (Default|ResetItemSlot _controllerref (Variables|Default|GetContainerType) Index))