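; Crafting component that loads a recipe list at BeginPlay from the DT_Crafting rows flagged craftable.
; Pressing H checks each recipe's ingredients against Inventory items by name and exact quantity, then calls Crafting if any check passes.
; The match counter is not reset between recipes, so matches accumulate across the list.
; Crafting itself is an empty stub.
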(event EventBeginPlay
  (CallFunction|InitCraftList))

(event Input|KeyboardEvents|H
  (params (Key :type Key%20Structure :default "None"))
  (:Pressed
    (bind _isavaiable (CallFunction|IsCraftingAvaiable))
    (if _isavaiable
      (CallFunction|Crafting))))

(fn InitCraftList
  (bind _outrownames (DataTable|GetDataTableRowNames "/Game/Inventory/Craft/DT_Crafting.DT_Crafting"))
  (for _array_element _outrownames
    (bind _returnvalue (Utilities|GetDataTableRow "/Game/Inventory/Craft/DT_Crafting.DT_Crafting" _array_element)
      (:then
        (if (.IsCraftble (Utilities|Struct|BreakS_CraftRecipe _returnvalue))
          (Utilities|Array|Add (Variables|Default|GetCraftList) _returnvalue))))))

(fn IsCraftingAvaiable
  (for _array_element (Variables|Default|GetCraftList)
    (for _array_element_2 (.Ingridient (Utilities|Struct|BreakS_CraftRecipe _array_element))
      (for _array_element_3 (Variables|/Game/Inventory/BP/BP_Inventory.BP_Inventory_C|GetItems (Variables|Default|GetInventory))
        (if (Utilities|Enum|Equal(Enum) (.Name (Utilities|Struct|BreakS_ItemStruct _array_element_3)) (Utilities|Text|ToText(Name) (.ID (Utilities|Struct|BreakS_Ingridient _array_element_2))))
          (if (== (.Quantitty (Utilities|Struct|BreakS_ItemStruct _array_element_3)) (.Amount (Utilities|Struct|BreakS_Ingridient _array_element_2)))
            (Math|Integer|IncrementInt (LocalVariables|GetMach))))))
    (LocalVariables|SetAvaiable (or (>= (LocalVariables|GetMach) (Utilities|Array|Length (.Ingridient (Utilities|Struct|BreakS_CraftRecipe _array_element)))) (LocalVariables|GetAvaiable))))
  (return (LocalVariables|GetAvaiable)))

(fn Crafting)