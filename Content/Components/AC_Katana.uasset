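; Katana combat component for BP_Kunaiji that handles equipping, attacking, blocking and blade damage.
; Equip and unequip snap the level's BP_BladeKatana between hand and holster sockets, gating attack and block input.
; Attacks cycle slash montages through a combo index, while block plays an idle montage and sets HasBlock.
; A looping timer box-traces between the blade's Tip and Base sockets while WeaponTrace is toggled on, applying rate-limited damage.
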(event Custom|KatanaTrace
  (if (Variables|Default|GetWeapon%20Trace)
    (bind _katana (Variables|Default|GetKatana)
      (:then
        (bind _mesh (Default|GetMesh _katana))
        (bind _outhit (Collision|BoxTraceByChannel (Transformation|GetSocketLocation _mesh "Tip") (Transformation|GetSocketLocation _mesh "Base") (Math|Vector|MakeVector (/ (Math|Vector|Distance(Vector) (Transformation|GetSocketLocation _mesh "Tip") (Transformation|GetSocketLocation _mesh "Base")) 2.0) 1e+02 5.0) (Math|Rotator|FindLookatRotation (Transformation|GetSocketLocation _mesh "Tip") (Transformation|GetSocketLocation _mesh "Base")) "TraceTypeQuery1" false 0 "None"))
        (Utilities|FlowControl|DoOnce false :!label _label
          (:Completed
            (Game|Damage|ApplyDamage (.HitActor (Collision|BreakHitResult _outhit)) 15.0 0 0)
            (Utilities|FlowControl|Delay 0.1)
            (goto _label Reset))))
      (:else))))

(event Custom|CharRef
  (bind _asbp_kunaiji (Utilities|Casting|CastToBP_Kunaiji (Components|GetOwner)))
  (Variables|Default|SetAs%20BP%20Kunaiji _asbp_kunaiji))

(event Custom|KatanaTimer
  (Utilities|Time|SetTimerbyEvent (delegate Custom|KatanaTrace) 0.01 true))

(event Custom|ResetAttack
  (bind _as_bp_kunaiji (Variables|Default|GetAs%20BP%20Kunaiji))
  (bind _mesh (Variables|/Script/Engine.Character|GetMesh _as_bp_kunaiji))
  ;[1 1 1] Attack
  (Utilities|FlowControl|DoOnce false) ; enters at Reset
)

(event Input|EnhancedActionEvents|EnhancedInputActionIA_Block
  (params (ActionValue :type Boolean) (ElapsedSeconds :type Float%20%28double-precision%29) (TriggeredSeconds :type Float%20%28double-precision%29) (InputAction :type Input%20Action%20Object%20Reference :default "/Game/Game/Input/InputAction/IA_Block.IA_Block"))
  (bind _as_bp_kunaiji (Variables|Default|GetAs%20BP%20Kunaiji))
  (bind _as_bp_kunaiji_2 (Variables|Default|GetAs%20BP%20Kunaiji))
  ;[1 1 1] Block
  (:Started
    (if (and (Variables|Default|GetEqKatana) (Variables|/Game/Character/BP_main/BP_Kunaiji.BP_Kunaiji_C|GetHas%20Sword? (Variables|Default|GetAs%20BP%20Kunaiji)))
      (Animation|PlayAnimMontage _as_bp_kunaiji_2 "/Game/Character/Animation/Fight/Block_Idle.Block_Idle" 1.0 "None")
      (Variables|/Game/Character/BP_main/BP_Kunaiji.BP_Kunaiji_C|SetHas%20Block _as_bp_kunaiji true)))
  (:Completed
    (Animation|StopAnimMontage _as_bp_kunaiji_2 "/Game/Character/Animation/Fight/Block_Idle.Block_Idle")
    (Variables|/Game/Character/BP_main/BP_Kunaiji.BP_Kunaiji_C|SetHas%20Block _as_bp_kunaiji false)))

(event Input|EnhancedActionEvents|EnhancedInputActionIA_Attack
  (params (ActionValue :type Boolean) (ElapsedSeconds :type Float%20%28double-precision%29) (TriggeredSeconds :type Float%20%28double-precision%29) (InputAction :type Input%20Action%20Object%20Reference :default "/Game/Game/Input/InputAction/IA_Attack.IA_Attack"))
  (bind _as_bp_kunaiji (Variables|Default|GetAs%20BP%20Kunaiji))
  (bind _mesh (Variables|/Script/Engine.Character|GetMesh _as_bp_kunaiji))
  ;[1 1 1] Attack
  (if (and (Variables|/Game/Character/BP_main/BP_Kunaiji.BP_Kunaiji_C|GetHas%20Sword? (Variables|Default|GetAs%20BP%20Kunaiji)) (Variables|Default|GetEqKatana))
    (Utilities|FlowControl|DoOnce false :!label _label
      (:Completed
        (switch int (Variables|Default|GetAttack%20Anim%20Num)
          (:Default
            (Animation|Montage|PlayMontage _mesh "/Game/Character/Animation/Fight/Sword_Slash_Down_Montage.Sword_Slash_Down_Montage" :!label _label_2
              (:then
                (Math|Integer|IncrementInt (Variables|Default|GetAttack%20Anim%20Num)
                  (:%20%20
                    (Utilities|FlowControl|RetriggerableDelay 3.0)
                    (Variables|Default|SetAttack%20Anim%20Num 0)
                    (goto _label Reset))))))
          (:0
            (goto _label_2))
          (:1
            (Animation|Montage|PlayMontage _mesh "/Game/Character/Animation/Fight/Sword_Slash_Up_Montage.Sword_Slash_Up_Montage"
              (:then
                (Variables|Default|SetAttack%20Anim%20Num 2))))
          (:2
            (Animation|Montage|PlayMontage _mesh "/Game/Character/Animation/Fight/Sword_Slash_Down_Montage.Sword_Slash_Down_Montage"
              (:then
                (Variables|Default|SetAttack%20Anim%20Num 0)))))))))

(event EventBeginPlay
  (CallFunction|CharRef)
  (CallFunction|KatanaTimer))

(event EventCallToggleWeaponTrace
  (params (WeaponTraceOn :type Boolean))
  (Variables|Default|SetWeapon%20Trace WeaponTraceOn))

(fn EquipKatana
  (if (Variables|/Game/Character/BP_main/BP_Kunaiji.BP_Kunaiji_C|GetHas%20Sword? (Variables|Default|GetAs%20BP%20Kunaiji))
    (bind _returnvalue (Actor|GetActorOfClass "/Game/Character/BP_main/BP_BladeKatana.BP_BladeKatana_C"))
    (bind _output_get (Variables|Default|SetKatana _returnvalue))
    (Transformation|AttachComponentToComponent _output_get (Variables|/Script/Engine.Character|GetMesh (Variables|Default|GetAs%20BP%20Kunaiji)) "HandSword" "SnapToTarget" "SnapToTarget" "KeepRelative" true)
    (Variables|Default|SetEqKatana true)))

(fn UnequipKatana
  (if (Variables|/Game/Character/BP_main/BP_Kunaiji.BP_Kunaiji_C|GetHas%20Sword? (Variables|Default|GetAs%20BP%20Kunaiji))
    (bind _returnvalue (Actor|GetActorOfClass "/Game/Character/BP_main/BP_BladeKatana.BP_BladeKatana_C"))
    (bind _output_get (Variables|Default|SetKatana _returnvalue))
    (Transformation|AttachComponentToComponent _output_get (Variables|/Script/Engine.Character|GetMesh (Variables|Default|GetAs%20BP%20Kunaiji)) "SwordPlace" "SnapToTarget" "SnapToTarget" "KeepRelative" true)
    (Variables|Default|SetEqKatana false)))

(fn WeaponTrace)

(fn GetMesh
  (return 0))