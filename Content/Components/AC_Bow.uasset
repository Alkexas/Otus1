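; Actor component for the BP_Kunaiji character that handles bow equipping, aiming and arrow firing.
; Equip and unequip move the BP_Bow found in the level between hand and storage sockets when the character has a bow.
; Aiming switches the character to controller-facing rotation, plays the draw montage and drives the bow's state.
; Arrows spawn attached to a socket, then detach and fire along the player camera's forward vector, or can be destroyed.
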(event Custom|AimBegin
  (bind _as_bp_kunaiji (Variables|Default|GetAs%20BP%20Kunaiji))
  (bind _charactermovement (Variables|/Script/Engine.Character|GetCharacterMovement _as_bp_kunaiji))
  ;[1 1 1] AimingBow
  (Variables|/Script/Engine.CharacterMovementComponent|SetbOrientRotationToMovement _charactermovement false)
  (Variables|/Script/Engine.CharacterMovementComponent|SetbUseControllerDesiredRotation _charactermovement true)
  (Animation|Montage|PlayMontage (Variables|/Script/Engine.Character|GetMesh (Variables|Default|GetAs%20BP%20Kunaiji)) "/Game/Character/Animation/Bow/Standing_Draw_Arrow_Montage.Standing_Draw_Arrow_Montage"
    (:then
      (Variables|/Game/Character/BP_main/BP_Bow.BP_Bow_C|SetBow%20States (Variables|Default|GetBow) "NewEnumerator1"))))

(event Custom|FireArrowBegin
  ;[1 1 1] FireArrow
  (bind _arrow (Variables|Default|GetArrow)
    (:then
      (Transformation|DetachFromActor _arrow "KeepWorld" "KeepWorld" "KeepWorld")
      (Default|Fire _arrow (Math|Vector|GetForwardVector (.Rotation (Pawn|GetPlayerViewPoint (Game|GetPlayerController 0)))))
      (Variables|/Game/Character/BP_main/BP_Bow.BP_Bow_C|SetBow%20States (Variables|Default|GetBow) "NewEnumerator2")
      (Utilities|FlowControl|Delay 0.6)
      (Variables|/Game/Character/BP_main/BP_Bow.BP_Bow_C|SetBow%20States (Variables|Default|GetBow) "NewEnumerator1"))
    (:else)))

(event Custom|AimEnd
  (bind _as_bp_kunaiji (Variables|Default|GetAs%20BP%20Kunaiji))
  (bind _charactermovement (Variables|/Script/Engine.Character|GetCharacterMovement _as_bp_kunaiji))
  ;[1 1 1] AimingBow
  (Variables|/Script/Engine.CharacterMovementComponent|SetbOrientRotationToMovement _charactermovement true)
  (Variables|/Script/Engine.CharacterMovementComponent|SetbUseControllerDesiredRotation _charactermovement false)
  (Animation|StopAnimMontage (Variables|Default|GetAs%20BP%20Kunaiji) "/Game/Character/Animation/Bow/Standing_Draw_Arrow_Montage.Standing_Draw_Arrow_Montage")
  (Variables|/Game/Character/BP_main/BP_Bow.BP_Bow_C|SetBow%20States (Variables|Default|GetBow) "NewEnumerator0"))

(event EventBeginPlay
  (bind _asbp_kunaiji (Utilities|Casting|CastToBP_Kunaiji (Components|GetOwner)))
  (Variables|Default|SetAs%20BP%20Kunaiji _asbp_kunaiji))

(fn EquipBow
  (if (Variables|/Game/Character/BP_main/BP_Kunaiji.BP_Kunaiji_C|GetHas%20Bow? (Variables|Default|GetAs%20BP%20Kunaiji))
    (bind _returnvalue (Actor|GetActorOfClass "/Game/Character/BP_main/BP_Bow.BP_Bow_C"))
    (bind _output_get (Variables|Default|SetBow _returnvalue))
    (Transformation|AttachComponentToComponent _output_get (Variables|/Script/Engine.Character|GetMesh (Variables|Default|GetAs%20BP%20Kunaiji)) "BowHand" "SnapToTarget" "SnapToTarget" "KeepRelative" true)
    (Variables|Default|SetEqBow true)))

(fn UnequipBow
  (if (Variables|/Game/Character/BP_main/BP_Kunaiji.BP_Kunaiji_C|GetHas%20Bow? (Variables|Default|GetAs%20BP%20Kunaiji))
    (bind _returnvalue (Actor|GetActorOfClass "/Game/Character/BP_main/BP_Bow.BP_Bow_C"))
    (bind _output_get (Variables|Default|SetBow _returnvalue))
    (Transformation|AttachComponentToComponent _output_get (Variables|/Script/Engine.Character|GetMesh (Variables|Default|GetAs%20BP%20Kunaiji)) "BowPlace" "SnapToTarget" "SnapToTarget" "KeepRelative" true)
    (Variables|Default|SetEqBow false)))

(fn SpawnArrow
  (bind _returnvalue (Game|SpawnActorfromClass "/Game/Character/BP_main/BP_Arrow.BP_Arrow_C" (Math|Transform|MakeTransform "0, 0, 0" "0, 0, 0" "1.000000,1.000000,1.000000") "Undefined" "MultiplyWithRoot" 0 (Variables|Default|GetAs%20BP%20Kunaiji)))
  (bind _output_get (Variables|Default|SetArrow _returnvalue))
  (Transformation|AttachComponentToComponent _output_get (Variables|/Script/Engine.Character|GetMesh (Variables|Default|GetAs%20BP%20Kunaiji)) "ArrowSlot" "SnapToTarget" "SnapToTarget" "SnapToTarget" true))

(fn DestroyArrow
  (bind _arrow (Variables|Default|GetArrow)
    (:then
      (Actor|DestroyActor _arrow))
    (:else)))