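; Actor component that handles sword combo attacks and blocking for its BP_Kunaiji owner.
; Attack input, with the sword equipped, passes a DoOnce gate and steps a counter through down, up and down slash montages.
; The first slash starts a retriggerable delay that resets counter and gate; ResetAttack also reopens the gate.
; Block input plays the block montage and sets HasBlock on the owner until released.
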(event Custom|Reset%20Attack
  (bind _as_bp_kunaiji (Variables|Default|GetAs%20BP%20Kunaiji))
  (bind _mesh (Variables|/Script/Engine.Character|GetMesh _as_bp_kunaiji))
  ;[1 1 1] Combo attack
  (Utilities|FlowControl|DoOnce false) ; enters at Reset
)

(event Input|EnhancedActionEvents|EnhancedInputActionIA_Block
  (params (ActionValue :type Boolean) (ElapsedSeconds :type Float%20%28double-precision%29) (TriggeredSeconds :type Float%20%28double-precision%29) (InputAction :type Input%20Action%20Object%20Reference :default "/Game/Game/Input/InputAction/IA_Block.IA_Block"))
  (bind _as_bp_kunaiji (Variables|Default|GetAs%20BP%20Kunaiji))
  (bind _as_bp_kunaiji_2 (Variables|Default|GetAs%20BP%20Kunaiji))
  (bind _as_bp_kunaiji_3 (Variables|Default|GetAs%20BP%20Kunaiji))
  ;[1 1 1] Block
  (:Started
    (if (Math|Boolean|ANDBoolean (Variables|/Game/Character/BP_main/BP_Kunaiji.BP_Kunaiji_C|GetIs%20Sword%20Equiped? _as_bp_kunaiji) (Variables|/Game/Character/BP_main/BP_Kunaiji.BP_Kunaiji_C|GetHas%20Sword? _as_bp_kunaiji) (not (Variables|/Game/Character/BP_main/BP_Kunaiji.BP_Kunaiji_C|GetIs%20Bow%20Equiped? _as_bp_kunaiji)))
      (Animation|PlayAnimMontage _as_bp_kunaiji_2 "/Game/Character/Animation/Fight/Block_Idle.Block_Idle" 1.0 "None")
      (Variables|/Game/Character/BP_main/BP_Kunaiji.BP_Kunaiji_C|SetHas%20Block _as_bp_kunaiji_3 true)))
  (:Completed
    (Animation|StopAnimMontage _as_bp_kunaiji_2 "/Game/Character/Animation/Fight/Block_Idle.Block_Idle")
    (Variables|/Game/Character/BP_main/BP_Kunaiji.BP_Kunaiji_C|SetHas%20Block _as_bp_kunaiji_3 false)))

(event Input|EnhancedActionEvents|EnhancedInputActionIA_Attack
  (params (ActionValue :type Boolean) (ElapsedSeconds :type Float%20%28double-precision%29) (TriggeredSeconds :type Float%20%28double-precision%29) (InputAction :type Input%20Action%20Object%20Reference :default "/Game/Game/Input/InputAction/IA_Attack.IA_Attack"))
  (bind _as_bp_kunaiji (Variables|Default|GetAs%20BP%20Kunaiji))
  (bind _as_bp_kunaiji_2 (Variables|Default|GetAs%20BP%20Kunaiji))
  (bind _mesh (Variables|/Script/Engine.Character|GetMesh _as_bp_kunaiji_2))
  ;[1 1 1] Combo attack
  (if (and (Variables|/Game/Character/BP_main/BP_Kunaiji.BP_Kunaiji_C|GetHas%20Sword? _as_bp_kunaiji) (Variables|/Game/Character/BP_main/BP_Kunaiji.BP_Kunaiji_C|GetIs%20Sword%20Equiped? _as_bp_kunaiji))
    (Utilities|FlowControl|DoOnce false :!label _label
      (:Completed
        (switch int (Variables|Default|GetAttack%20Anim%20Num)
          (:Default
            (Animation|Montage|PlayMontage _mesh "/Game/Character/Animation/Fight/Sword_Slash_Down_Montage.Sword_Slash_Down_Montage" :!label _label_2
              (:then
                (Math|Integer|IncrementInt (Variables|Default|GetAttack%20Anim%20Num)
                  (:%20%20
                    (Utilities|FlowControl|RetriggerableDelay 3.0)
                    (Variables|Default|SetAttack%20Anim%20Num 0)
                    (goto _label Reset))))))
          (:0
            (goto _label_2))
          (:1
            (Animation|Montage|PlayMontage _mesh "/Game/Character/Animation/Fight/Sword_Slash_Up_Montage.Sword_Slash_Up_Montage"
              (:then
                (Variables|Default|SetAttack%20Anim%20Num 2))))
          (:2
            (Animation|Montage|PlayMontage _mesh "/Game/Character/Animation/Fight/Sword_Slash_Down_Montage.Sword_Slash_Down_Montage"
              (:then
                (Variables|Default|SetAttack%20Anim%20Num 0)))))))))

(event EventBeginPlay
  (bind _asbp_kunaiji (Utilities|Casting|CastToBP_Kunaiji (Components|GetOwner)))
  (Variables|Default|SetAs%20BP%20Kunaiji _asbp_kunaiji))