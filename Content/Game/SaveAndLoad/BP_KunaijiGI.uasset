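; Game instance for Kunaiji that owns the game's save data and handles loading and saving it.
; On Init it synchronously loads the BP_SaveGame object from its slot into GameData, creating a new one if no save exists.
; Load and save events each offer sync or async paths.
; SavePlayerData writes player data into GameData before saving, and GetGameData exposes the cached object.
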(event EventLoadDataGame
  (params (Async :type Boolean))
  ;[0 1 0.04728] Load
  (bind _returnvalue (SaveGame|DoesSaveGameExist (Variables|Default|GetSlot%20Name)))
  (if _returnvalue
    (if Async
      (bind _savegame (|AsyncLoadGamefromSlot (Variables|Default|GetSlot%20Name))
        (:Completed
          (bind _asbp_save_game (Utilities|Casting|CastToBP_SaveGame _savegame))
          (Variables|Default|SetGameData _asbp_save_game)))
      (else
        (bind _returnvalue_2 (SaveGame|LoadGamefromSlot (Variables|Default|GetSlot%20Name)))
        (bind _asbp_save_game_2 (Utilities|Casting|CastToBP_SaveGame _returnvalue_2))
        (Variables|Default|SetGameData _asbp_save_game_2)))
    (else
      (bind _returnvalue_3 (SaveGame|CreateSaveGameObject "/Game/Game/SaveAndLoad/BP_SaveGame.BP_SaveGame_C"))
      (Variables|Default|SetGameData _returnvalue_3))))

(event EventSaveDataGame
  (params (Async :type Boolean))
  ;[1 1 1] Save
  (if Async
    (|AsyncSaveGametoSlot (Variables|Default|GetGameData) (Variables|Default|GetSlot%20Name))
    (else
      (SaveGame|SaveGametoSlot (Variables|Default|GetGameData) (Variables|Default|GetSlot%20Name)))))

(event EventSavePlayerData
  (params (PlayerData :type S%20Player%20Data%20Structure) (Async :type Boolean))
  (Variables|/Game/Game/SaveAndLoad/BP_SaveGame.BP_SaveGame_C|SetPlayerData (Variables|Default|GetGameData) PlayerData)
  (CallFunction|SaveDataGame Async))

(event EventInit
  (CallFunction|LoadDataGame false))

(fn GetGameData
  (return (Variables|Default|GetGameData)))