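; BP_ExplosiveBarrel is a barrel actor that explodes shortly after something overlaps its Cylinder component.
; The overlap destroys the Cylinder, reveals ZoneDamage, then after a short delay applies full radial damage with a particle effect, sound and RadialForce impulse.
; ZoneDamage is then removed, and a second delay precedes destroying the emitter and actor.
; GetMesh and the construction script are empty.
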(event OnComponentBeginOverlap(Cylinder)
  (params (OverlappedComponent :type Primitive%20Component%20Object%20Reference) (OtherActor :type Actor%20Object%20Reference) (OtherComp :type Primitive%20Component%20Object%20Reference) (OtherBodyIndex :type Integer) (bFromSweep :type Boolean) (SweepResult :type Hit%20Result%20Structure%20%28by%20ref%29))
  (bind _returnvalue (Transformation|GetActorLocation))
  (Components|DestroyComponent (Variables|Default|GetCylinder))
  (Rendering|SetVisibility (Variables|Default|GetZoneDamage) true false)
  (Utilities|FlowControl|Delay 1.5)
  (Game|Damage|ApplyRadialDamage 1e+02 _returnvalue 5e+02 0 0 self 0 true "ECC_Visibility")
  (bind _returnvalue_2 (Effects|SpawnEmitteratLocation "/Engine/Tutorial/SubEditors/TutorialAssets/TutorialParticleSystem.TutorialParticleSystem" _returnvalue))
  (Audio|PlaySoundatLocation "/Game/DynamicGrassLite/Blueprints/InternalLogic/FirstPersonBP/Audio/FirstPersonTemplateWeaponFire02.FirstPersonTemplateWeaponFire02" _returnvalue "0, 0, 0" 1.0 1.0 0.0 0 0 0 0)
  (Class|RadialForceComponent|FireImpulse (Variables|Default|GetRadialForce))
  (Components|DestroyComponent (Variables|Default|GetZoneDamage))
  (Utilities|FlowControl|Delay 5.0)
  (Components|DestroyComponent _returnvalue_2)
  (Actor|DestroyActor))

(fn ConstructionScript)

(fn GetMesh
  (return 0))