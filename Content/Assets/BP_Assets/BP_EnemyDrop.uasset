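; BP_EnemyDrop spawns an item, apparently a key, once every enemy in its melee and ranged bot lists is dead.
; On BeginPlay it caches BP_Kunaiji, counts both lists and binds to each bot's death event.
; Each death decrements its counter, setting a flag at zero.
; A looping timer polls both flags, then spawns BP_Item once at an offset from Kunaiji and plays the key sound.
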(event Custom|EnemyDead
  (bind _result (Math|Integer|DecrementInt (Variables|Default|GetIndexEnemy))
    (:%20%20
      (if (<= _result 0)
        (Variables|Default|SetMelee true)))))

(event Custom|RangeDead
  (bind _result (Math|Integer|DecrementInt (Variables|Default|GetIndexEnemyRange))
    (:%20%20
      (if (<= _result 0)
        (Variables|Default|SetRange true)))))

(event Custom|SpawnKey
  (bind _kunajiref (Variables|Default|GetKunajiRef))
  (bind _rootcomponent (Variables|/Script/Engine.Actor|GetRootComponent _kunajiref))
  (bind _returnvalue (Transformation|GetWorldLocation _rootcomponent))
  (bind _returnvalue_2 (Transformation|GetWorldRotation _rootcomponent))
  (bind _returnvalue_3 (* _returnvalue_2 1e+02))
  (bind _returnvalue_4 (+ _returnvalue _returnvalue_3))
  (if (and (Variables|Default|GetMelee) (Variables|Default|GetRange))
    (Utilities|FlowControl|DoOnce false
      (:Completed
        (Game|SpawnActorfromClass "/Game/Inventory/BP/BP_Item.BP_Item_C" (Math|Transform|MakeTransform _returnvalue_4 "0, 0, 0" "1.000000,1.000000,1.000000") "Undefined" "MultiplyWithRoot" 0 (Variables|Default|GetItem) 0)
        (Audio|PlaySoundatLocation "/Game/Sound/Assets/SC_Key.SC_Key" _returnvalue_4 "0, 0, 0" 1.0 1.0 0.0 0 0 0 0)))))

(event Custom|BotCount
  (bind _botmelee (Variables|Default|GetBotMelee))
  (bind _botrange (Variables|Default|GetBotRange))
  (Utilities|FlowControl|Sequence
    (:then_0
      (Variables|Default|SetIndexEnemy (Utilities|Array|Length _botmelee))
      (for _array_element _botmelee
        (EventDispatchers|BindEventtoMeleeDeath _array_element (delegate Custom|EnemyDead))))
    (:then_1
      (Variables|Default|SetIndexEnemyRange (Utilities|Array|Length _botrange))
      (for _array_element_2 _botrange
        (EventDispatchers|BindEventtoRangeDeath _array_element_2 (delegate Custom|RangeDead))))
    (:then_2
      (Utilities|Time|SetTimerbyEvent (delegate Custom|SpawnKey) 0.1 true true))))

(event Custom|CharacterRef
  (bind _returnvalue (Actor|GetActorOfClass "/Game/Character/BP_main/BP_Kunaiji.BP_Kunaiji_C"))
  (Variables|Default|SetKunajiRef _returnvalue))

(event EventBeginPlay
  (CallFunction|CharacterRef)
  (CallFunction|BotCount))

(fn ConstructionScript)