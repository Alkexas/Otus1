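; Interactable double-door gate that opens once the player holds four keys.
; Interact scans BP_Kunaiji's BPInventory for a Key quantity of exactly four, then uses the IsOpen flag to trigger opening only once.
; Opening disables player input for a fixed delay while playing a sound and camera shake.
; Timelines swing both doors on yaw, with the right driven from the left's update, which also fires the GateOpen dispatcher.
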(event Custom|OpenGate
  ;[1 0.8963 0] Open
  (CallFunction|InputDisEn)
  (CallFunction|SoundandShake)
  (bind _door (Timeline|LeftOpen Play)
    (:Update
      (Transformation|SetRelativeRotation (Variables|Default|GetLeftDoor) (Math|Rotator|MakeRotator 0.0 0.0 _door) false false)
      (bind _door_2 (Timeline|RightOpen Play)
        (:Update
          (Transformation|SetRelativeRotation (Variables|Default|GetRightDoor) (Math|Rotator|MakeRotator 0.0 0.0 _door_2) false false)
          (Default|CallGateOpen))))))

(event Custom|SoundAndShake
  ;[1 0.8947 0] Sound and Shake
  (Audio|PlaySound2D "/Game/Sound/Assets/SC_GateOpen.SC_GateOpen" 1.0 1.0 0.0 0 0)
  (Class|LegacyCameraShake|StartLegacyCameraShake (Game|GetPlayerCameraManager 0) "/Game/Assets/Gate/BP_GateShake.BP_GateShake_C" 1.0 "CameraLocal" "0, 0, 0"))

(event Custom|HasKey
  ;[0 0.2679 1] Find Key
  (bind _outactors (Actor|GetAllActorsOfClass "/Game/Character/BP_main/BP_Kunaiji.BP_Kunaiji_C"))
  (bind _output_get (Variables|Default|SetBP%20Inventory (Variables|/Game/Character/BP_main/BP_Kunaiji.BP_Kunaiji_C|GetBP_Inventory (Utilities|Array|Get(acopy) _outactors))))
  (for _array_element (Variables|/Game/Inventory/BP/BP_Inventory.BP_Inventory_C|GetItems _output_get)
    (if (Utilities|Enum|Equal(Enum) (.name _array_element) (Variables|Default|GetKey))
      (bind _output_get_2 (Variables|Default|SetCurrentKey (.quantitty _array_element)))
      (if (== _output_get_2 4)
        (Variables|Default|SetHasKey? true)
        (Variables|Default|SetCurrentKey 0)))))

(event Custom|InputDisEn
  ;[1 0 0] Input (Dis-En)
  (Input|DisableInput (Game|GetPlayerCharacter 0) (Game|GetPlayerController 0))
  (Utilities|FlowControl|Delay 5.0)
  (Input|EnableInput (Game|GetPlayerCharacter 0) (Game|GetPlayerController 0)))

(fn ConstructionScript)

(fn Interact
  (params (IsPickUp? :type Boolean))
  (CallFunction|HasKey)
  (if (Variables|Default|GetHasKey?)
    (if (Variables|Default|GetIsOpen?)
      (Variables|Default|SetIsOpen? false)
      (CallFunction|OpenGate)
      (return false))))