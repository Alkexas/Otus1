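; BP_Spawner is a one-shot trigger that spawns melee and ranged enemy bots when an actor tagged Character enters its sphere.
; It spawns set counts of BP_BotMelee and BP_BotRange at reachable navmesh points near random locations in its box, storing each type in an array.
; It then calls EnemySpawned.
; On BeginPlay it caches the player's BP_Kunaiji, which these graphs never use.
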(event OnComponentBeginOverlap(Sphere)
  (params (OverlappedComponent :type Primitive%20Component%20Object%20Reference) (OtherActor :type Actor%20Object%20Reference) (OtherComp :type Primitive%20Component%20Object%20Reference) (OtherBodyIndex :type Integer) (bFromSweep :type Boolean) (SweepResult :type Hit%20Result%20Structure%20%28by%20ref%29))
  (if (Actor|ActorHasTag OtherActor "Character")
    (Utilities|FlowControl|DoOnce false
      (:Completed
        (CallFunction|Spawner)
        (Default|CallEnemySpawned)))))

(event Custom|Spawner
  (bind _box (Variables|Default|GetBox))
  (bind _returnvalue (Components|Box|GetScaledBoxExtent _box))
  (bind _relativelocation (Variables|/Script/Engine.SceneComponent|GetRelativeLocation _box))
  (bind _returnvalue_2 (Math|Random|RandomPointinBoundingBox _relativelocation _returnvalue))
  (bind _randomlocation (AI|Navigation|GetRandomReachablePointinRadius _returnvalue_2 1.5e+03 0 0))
  (Utilities|FlowControl|Sequence
    (:then_0
      (for _index (range 1 (Variables|Default|GetBotMeleeCount))
        (bind _returnvalue_3 (Game|SpawnActorfromClass "/Game/AI/BP_BotMelee.BP_BotMelee_C" (Math|Transform|MakeTransform _randomlocation "0, 0, 0" "1.000000,1.000000,1.000000") "AlwaysSpawn" "MultiplyWithRoot" 0 0))
        (Utilities|Array|Add (Variables|Default|GetMeleeArray) _returnvalue_3)
        (Variables|Default|SetMeleeArray (Variables|Default|GetMeleeArray))))
    (:then_1
      (for _index_2 (range 1 (Variables|Default|GetBotRangeCount))
        (bind _returnvalue_4 (Game|SpawnActorfromClass "/Game/AI/BP_BotRange.BP_BotRange_C" (Math|Transform|MakeTransform _randomlocation "0, 0, 0" "1.000000,1.000000,1.000000") "AlwaysSpawn" "MultiplyWithRoot" 0 0))
        (Utilities|Array|Add (Variables|Default|GetRangeArray) _returnvalue_4)
        (Variables|Default|SetRangeArray (Variables|Default|GetRangeArray))))))

(event Custom|KunajuRef
  (bind _asbp_kunaiji (Utilities|Casting|CastToBP_Kunaiji (Game|GetPlayerCharacter 0)))
  (Variables|Default|SetAs%20BP%20Kunaiji _asbp_kunaiji))

(event EventBeginPlay
  (CallFunction|KunajuRef))

(fn ConstructionScript)