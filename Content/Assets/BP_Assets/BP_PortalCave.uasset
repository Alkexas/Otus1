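; BP_PortalCave is a trigger portal that moves the player between streamed levels when BP_Kunaiji overlaps its Box.
; On overlap it shows WB_LoadingScreen, streams in LevelLoad, teleports the player character to TeleportPoint, then unloads CurrentLevel.
; It then plays the SC_CaveNoise sound and removes the loading screen after a short delay.
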(event OnComponentBeginOverlap(Box)
  (params (OverlappedComponent :type Primitive%20Component%20Object%20Reference) (OtherActor :type Actor%20Object%20Reference) (OtherComp :type Primitive%20Component%20Object%20Reference) (OtherBodyIndex :type Integer) (bFromSweep :type Boolean) (SweepResult :type Hit%20Result%20Structure%20%28by%20ref%29))
  (Utilities|Casting|CastToBP_Kunaiji OtherActor)
  (bind _returnvalue (UserInterface|CreateWidget "/Game/UI/WB_LoadingScreen.WB_LoadingScreen_C"))
  (UserInterface|Viewport|AddtoViewport _returnvalue 0)
  (Variables|Default|SetLoading%20Widget _returnvalue)
  (Class|GameplayStatics|LoadStreamLevelbySoftObjectPtr (Variables|Default|GetLevelLoad) true false)
  (Transformation|SetActorLocation (Game|GetPlayerCharacter 0) (Transformation|GetWorldLocation (Variables|Default|GetTeleportPoint)) false true)
  (Class|GameplayStatics|UnloadStreamLevelbySoftObjectPtr (Variables|Default|GetCurrentLevel) false)
  (Audio|PlaySound2D "/Game/Sound/Nature/SC_CaveNoise.SC_CaveNoise" 1.0 1.0 0.0 0 0)
  (Utilities|FlowControl|Delay 1.5)
  (Widget|RemovefromParent (Variables|Default|GetLoading%20Widget)))

(fn ConstructionScript)