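; BP_Cinematic is an actor with a skeletal mesh that is positioned along a referenced spline path, apparently for cinematics.
; SetPositionState forwards a position to EventMove, which makes the mesh visible and moves the actor.
; The position scales the spline length to give the world-space location, while rotation is always sampled at the spline's end rather than at the current distance.
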(event Custom|EventMove
  (params (Positon :type Float%20%28double-precision%29))
  (bind _splitepath (Variables|Default|GetSplitePath))
  (bind _spline (Variables|/Game/Assets/BP_Assets/BP_Spline.BP_Spline_C|GetSpline _splitepath))
  (bind _returnvalue (Spline|GetSplineLength _spline))
  (Rendering|SetVisibility (Variables|Default|GetSkeletalMesh) true false)
  (Transformation|SetActorLocationAndRotation (Spline|GetLocationatDistanceAlongSpline _spline (* Positon _returnvalue) "World") (Spline|GetRotationatDistanceAlongSpline _spline _returnvalue "World")))

(fn ConstructionScript)

(fn SetPositionState
  (params (Position :type Float%20%28double-precision%29))
  (CallFunction|EventMove Position))