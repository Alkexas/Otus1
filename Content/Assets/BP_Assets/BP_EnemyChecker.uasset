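; BP_EnemyChecker watches a spawner's enemies and rewards clearing them by spawning a key item near the player, BP_Kunaiji, with a sound.
; On the spawner's EnemySpawned event, it gathers melee and ranged bots and binds their death events.
; Each death decrements that type's leftover loop index, setting a cleared flag below zero.
; A looping timer polls both flags and spawns the item through a DoOnce.
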(event Custom|SpawnKey
  (bind _kunajiref (Variables|Default|GetKunajiRef))
  (bind _rootcomponent (Variables|/Script/Engine.Actor|GetRootComponent _kunajiref))
  (bind _returnvalue (Transformation|GetWorldLocation _rootcomponent))
  (bind _returnvalue_2 (Transformation|GetWorldRotation _rootcomponent))
  (bind _returnvalue_3 (* _returnvalue_2 1e+02))
  (bind _returnvalue_4 (+ _returnvalue _returnvalue_3))
  (if (and (Variables|Default|GetMelee) (Variables|Default|GetRange))
    (Utilities|FlowControl|DoOnce false
      (:Completed
        (Game|SpawnActorfromClass "/Game/Inventory/BP/BP_Item.BP_Item_C" (Math|Transform|MakeTransform _returnvalue_4 "0, 0, 0" "1.000000,1.000000,1.000000") "Undefined" "MultiplyWithRoot" 0 (Variables|Default|GetItem) 0)
        (Audio|PlaySoundatLocation "/Engine/VREditor/Sounds/UI/Camera_Shutter.Camera_Shutter" _returnvalue_4 "0, 0, 0" 1.0 1.0 0.0 0 0 0 0)))))

(event Custom|BotCount
  (Utilities|FlowControl|Sequence
    (:then_0
      (for _array_element (Variables|/Game/Assets/BP_Assets/BP_Spawner.BP_Spawner_C|GetMeleeArray (Variables|Default|GetSpawner))
        (bind _asbp_bot_melee (Utilities|Casting|CastToBP_BotMelee _array_element))
        (Utilities|Array|Add (Variables|Default|GetBotMelee) _asbp_bot_melee)
        (bind _output_get (Variables|Default|SetBotMelee (Variables|Default|GetBotMelee)))
        (for (_array_element_2 _array_index) _output_get
          (EventDispatchers|BindEventtoMeleeDeath _array_element_2 (delegate Custom|CustomEvent)))))
    (:then_1
      (for _array_element_3 (Variables|/Game/Assets/BP_Assets/BP_Spawner.BP_Spawner_C|GetRangeArray (Variables|Default|GetSpawner))
        (bind _asbp_bot_range (Utilities|Casting|CastToBP_BotRange _array_element_3))
        (Utilities|Array|Add (Variables|Default|GetBotRange) _asbp_bot_range)
        (bind _output_get_2 (Variables|Default|SetBotRange (Variables|Default|GetBotRange)))
        (for (_array_element_4 _array_index_2) _output_get_2
          (EventDispatchers|BindEventtoRangeDeath _array_element_4 (delegate Custom|CustomEvent_1)))))
    (:then_2
      (Utilities|Time|SetTimerbyEvent (delegate Custom|SpawnKey) 0.1 true true))))

(event Custom|CharacterRef
  (bind _returnvalue (Actor|GetActorOfClass "/Game/Character/BP_main/BP_Kunaiji.BP_Kunaiji_C"))
  (Variables|Default|SetKunajiRef _returnvalue))

(event Custom|CustomEvent_1
  (bind _result (Math|Integer|DecrementInt (stale Custom|BotCount _array_index_2))
    (:%20%20
      (if (< _result 0)
        (Variables|Default|SetRange true)))))

(event Custom|CustomEvent
  (bind _result (Math|Integer|DecrementInt (stale Custom|BotCount _array_index))
    (:%20%20
      (if (< _result 0)
        (Variables|Default|SetMelee true)))))

(event EventBeginPlay
  (CallFunction|CharacterRef)
  (EventDispatchers|BindEventtoEnemySpawned (Variables|Default|GetSpawner) (delegate Custom|BotCount)))

(fn ConstructionScript)