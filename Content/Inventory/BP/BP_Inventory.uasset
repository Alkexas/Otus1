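; Player inventory with a fixed set of slots, loaded from and auto-saved to the game data held by BP_KunaijiGI.
; Interact sphere-traces near the player's feet for a BP_Item, stacks it up to a cap or fills an empty slot in array order, then destroys it.
; Each pickup refreshes WB_Inventory and fires an update event that writes the save slot.
; Tab toggles the widget, mouse cursor and input mode.
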(event Custom|AutoSaveInv
  (CallFunction|SaveInv))

(event Input|EnhancedActionEvents|EnhancedInputActionIA_Interact
  (params (ActionValue :type Boolean) (ElapsedSeconds :type Float%20%28double-precision%29) (TriggeredSeconds :type Float%20%28double-precision%29) (InputAction :type Input%20Action%20Object%20Reference :default "/Game/Game/Input/InputAction/IA_Interact.IA_Interact"))
  (bind _returnvalue (Game|GetPlayerCharacter 0))
  (bind _returnvalue_2 (Transformation|GetActorLocation _returnvalue))
  (bind _returnvalue_3 (- _returnvalue_2 "0.000000,0.000000,65.000000"))
  (bind _outhit (Collision|SphereTraceByChannel _returnvalue_3 _returnvalue_3 1.2e+02 "TraceTypeQuery1" false 0 "None"))
  (bind _asbp_item (Utilities|Casting|CastToBP_Item (.HitActor (Collision|BreakHitResult _outhit))))
  (for (_array_element _array_index) (Variables|Default|GetItems)
    (Utilities|IsValid _asbp_item
      (:Is%20Valid
        (if (Math|Boolean|ANDBoolean (Utilities|Enum|Equal(Enum) (.Name (Utilities|Struct|BreakS_ItemStruct _array_element)) (.Name (Utilities|Struct|BreakS_ItemStruct (Variables|/Game/Inventory/BP/BP_Item.BP_Item_C|GetItem _asbp_item)))) (.Stackable (Utilities|Struct|BreakS_ItemStruct (Variables|/Game/Inventory/BP/BP_Item.BP_Item_C|GetItem _asbp_item))) (<= (+ (.Quantitty (Utilities|Struct|BreakS_ItemStruct _array_element)) (.Quantitty (Utilities|Struct|BreakS_ItemStruct (Variables|/Game/Inventory/BP/BP_Item.BP_Item_C|GetItem _asbp_item)))) 30))
          (Utilities|Array|SetArrayElem (Variables|Default|GetItems) _array_index (Utilities|Struct|MakeS_ItemStruct (.Name (Utilities|Struct|BreakS_ItemStruct (Variables|/Game/Inventory/BP/BP_Item.BP_Item_C|GetItem _asbp_item))) (.Stackable (Utilities|Struct|BreakS_ItemStruct (Variables|/Game/Inventory/BP/BP_Item.BP_Item_C|GetItem _asbp_item))) (+ (.Quantitty (Utilities|Struct|BreakS_ItemStruct _array_element)) (.Quantitty (Utilities|Struct|BreakS_ItemStruct (Variables|/Game/Inventory/BP/BP_Item.BP_Item_C|GetItem _asbp_item)))) (.Thumbnail (Utilities|Struct|BreakS_ItemStruct (Variables|/Game/Inventory/BP/BP_Item.BP_Item_C|GetItem _asbp_item))) (.Mesh (Utilities|Struct|BreakS_ItemStruct (Variables|/Game/Inventory/BP/BP_Item.BP_Item_C|GetItem _asbp_item)))))
          (Default|LoadInventory (Variables|Default|GetInventoryWidget) self :!label _label)
          (Default|CallSaveInventoryUpdate)
          (Actor|DestroyActor _asbp_item)
          (elif (== (.Quantitty (Utilities|Struct|BreakS_ItemStruct _array_element)) 0)
            (Utilities|Array|SetArrayElem (Variables|Default|GetItems) _array_index (Variables|/Game/Inventory/BP/BP_Item.BP_Item_C|GetItem _asbp_item))
            (goto _label)))))))

(event EventBeginPlay
  (CallFunction|LoadInv)
  (bind _returnvalue (UserInterface|CreateWidget "/Game/Inventory/Widgets/WB_Inventory.WB_Inventory_C"))
  (Variables|Default|SetInventoryWidget _returnvalue)
  (Utilities|Array|Resize (Variables|Default|GetItems) 10)
  (Default|LoadInventory (Variables|Default|GetInventoryWidget) self)
  (EventDispatchers|BindEventtoSaveInventoryUpdate (delegate Custom|AutoSaveInv)))

(event Input|KeyboardEvents|Tab
  (params (Key :type Key%20Structure))
  (bind _returnvalue (Game|GetPlayerController 0))
  (bind _inventorywidget (Variables|Default|GetInventoryWidget))
  (:Pressed
    (if (Widget|IsVisible _inventorywidget)
      (Widget|RemovefromParent _inventorywidget)
      (Variables|/Script/Engine.PlayerController|SetbShowMouseCursor _returnvalue false)
      (Input|SetInputModeGameOnly _returnvalue false)
      (else
        (UserInterface|Viewport|AddtoViewport _inventorywidget 0)
        (Variables|/Script/Engine.PlayerController|SetbShowMouseCursor _returnvalue true)
        (Input|SetInputModeGameandUI _returnvalue 0 "DoNotLock" true false)))))

(fn SaveInv
  (bind _asbp_kunaiji_gi (Utilities|Casting|CastToBP_KunaijiGI (Game|GetGameInstance)))
  (Variables|/Game/Game/SaveAndLoad/BP_SaveGame.BP_SaveGame_C|SetItemStruct (Variables|/Game/Game/SaveAndLoad/BP_KunaijiGI.BP_KunaijiGI_C|GetGameData _asbp_kunaiji_gi) (Variables|Default|GetItems))
  (SaveGame|SaveGametoSlot (Variables|/Game/Game/SaveAndLoad/BP_KunaijiGI.BP_KunaijiGI_C|GetGameData _asbp_kunaiji_gi) (LocalVariables|GetNewLocalVar)))

(fn LoadInv
  (bind _asbp_kunaiji_gi (Utilities|Casting|CastToBP_KunaijiGI (Game|GetGameInstance)))
  (Variables|Default|SetItems (Variables|/Game/Game/SaveAndLoad/BP_SaveGame.BP_SaveGame_C|GetItemStruct (Variables|/Game/Game/SaveAndLoad/BP_KunaijiGI.BP_KunaijiGI_C|GetGameData _asbp_kunaiji_gi))))